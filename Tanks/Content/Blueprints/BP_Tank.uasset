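; BP_Tank is a player-input tank Blueprint with click-to-move driving, firing, track dust and engine audio.
; The Move input sends TankMovement to the mouse position through Tracks, bound at BeginPlay, and Fire calls the tank's Fire function.
; Tick toggles both dust emitters while moving, and calls IsCloseToDestination, which, despite its name, plays or reverses a timeline driving audio pitch by track acceleration.
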(event `self.ReceiveBeginPlay`
  (`TankMovementComponent.Initialise` (`self.TankMovement`) (`self.Tracks`)))

(event `self.ReceiveTick`
  (params (DeltaSeconds :type "Float (single-precision)"))
  (bind _rightdust (`self.RightDust`))
  (`self.Event Is Close To Destination`)
  ;[1 1 1] Dust particle system
  (if (`TankMovementComponent.IsMoving` (`self.TankMovement`))
    (`ActorComponent.Activate` _rightdust false)
    (`ActorComponent.Activate` (`self.LeftDust`) false)
    (else
      (`ActorComponent.Deactivate` _rightdust)
      (`ActorComponent.Deactivate` (`self.LeftDust`)))))

(event `Event Is Close To Destination`
  ;[1 1 1] Acceleration sound
  (if (`TankTracks.IsAccelerating` (`self.Tracks`))
    (bind (_direction _soundpitch) (`Timeline|Timeline_0` :!label _label)
      (:`Update`
        (`AudioComponent.SetPitchMultiplier` (`self.Audio`) _soundpitch)))
    (else
      (goto _label :!via `Reverse`))))

(event `InputAction|Move`
  (params (Key :type "Key Structure"))
  (:`Pressed`
    (`TankMovementComponent.MoveToMousePosition` (`self.TankMovement`))))

(event `InputAction|Fire`
  (params (Key :type "Key Structure"))
  (:`Pressed`
    (`self.Fire`)))

(fn `UserConstructionScript`)